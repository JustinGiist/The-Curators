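; Display case actor whose particle effect is tinted per level: Tutorial, Level 1, Level 2 or Level 3.
; The construction script switches on DisplayCaseEnum and sets the ParticleColor1 and ParticleColor2 color parameters on the DisplayCase component from that level's pair of color variables.
; All logic runs at construction, as the event graph holds only disabled default events.
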(event EventBeginPlay)

(event Collision|EventActorBeginOverlap
  (params (OtherActor :type Actor%20Object%20Reference)))

(event EventTick
  (params (DeltaSeconds :type Float%20%28single-precision%29)))

(fn ConstructionScript
  (bind _displaycase (Variables|Default|GetdisplayCase))
  (bind _displaycase_2 (Variables|Default|GetdisplayCase))
  (bind _displaycase_3 (Variables|Default|GetdisplayCase))
  (bind _displaycase_4 (Variables|Default|GetdisplayCase))
  (switch Utilities|FlowControl|Switch|SwitchondisplayCaseEnum (Variables|Default|GetdisplayCaseEnum)
    (:NewEnumerator1
      (Effects|Components|ParticleSystem|SetColorParameter _displaycase "ParticleColor1" (stale _output_get))
      (Effects|Components|ParticleSystem|SetColorParameter _displaycase "ParticleColor2" (stale _output_get)))
    (:NewEnumerator2
      (Effects|Components|ParticleSystem|SetColorParameter _displaycase_2 "ParticleColor1" (stale _output_get))
      (Effects|Components|ParticleSystem|SetColorParameter _displaycase_2 "ParticleColor2" (stale _output_get)))
    (:NewEnumerator3
      (Effects|Components|ParticleSystem|SetColorParameter _displaycase_3 "ParticleColor1" (stale _output_get))
      (Effects|Components|ParticleSystem|SetColorParameter _displaycase_3 "ParticleColor2" (stale _output_get)))
    (:NewEnumerator4
      (Effects|Components|ParticleSystem|SetColorParameter _displaycase_4 "ParticleColor1" (stale _output_get))
      (Effects|Components|ParticleSystem|SetColorParameter _displaycase_4 "ParticleColor2" (stale _output_get)))))