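; GreenDoor is an interactive door Blueprint that the player opens and closes with E while inside its DoorCollision volume.
; Overlap begin and end enable and disable input for player controller 0, without checking which actor overlaps.
; Each press flips DoorStatus and plays or reverses a timeline that slides Door2b by relative location, despite comments describing rotation.
; Unlock sound nodes are disconnected, and CheckInventory is an unused stub returning false.
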(event OnComponentEndOverlap(DoorCollision)
  (params (OtherActor :type Actor%20Object%20Reference) (OtherComp :type Primitive%20Component%20Object%20Reference) (OtherBodyIndex :type Integer))
  ;[1 1 1] If player is within Door Collision: Enable them to hit E(X button on 360 pad) and the door will rotate open
  (Input|DisableInput (Game|GetPlayerController 0)))

(event OnComponentBeginOverlap(DoorCollision)
  (params (OtherActor :type Actor%20Object%20Reference) (OtherComp :type Primitive%20Component%20Object%20Reference) (OtherBodyIndex :type Integer) (bFromSweep :type Boolean) (SweepResult :type Hit%20Result%20Structure%20%28by%20ref%29))
  ;[1 1 1] If player is within Door Collision: Enable them to hit E(X button on 360 pad) and the door will rotate open
  (Input|EnableInput (Game|GetPlayerController 0)))

(event Input|KeyboardEvents|E
  ;[1 1 1] On input rotate door
  (:Pressed
    (if (Variables|Default|Getdoor%20status)
      (Variables|Default|Setdoor%20status false)
      (bind _door_swipe (Timeline|Timeline_0 Play)
        (:Update
          (Transformation|SetRelativeLocation (Variables|Default|Getdoor2b) _door_swipe false)))
      (else
        (Variables|Default|Setdoor%20status true)
        (Timeline|Timeline_0 Reverse)))))

(fn ConstructionScript)

(fn CheckInventory
  (params (Item :type String))
  (return false))