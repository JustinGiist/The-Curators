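; Long display case prop Blueprint whose particle effect is color-themed by level.
; The construction script switches on an enum choice of Tutorial or one of three levels and sets the particle system's two color parameters from that level's pair of color variables.
; Disconnected setter nodes for those color variables never run, and the event graph holds no active logic.
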(event EventBeginPlay)

(event Collision|EventActorBeginOverlap
  (params (OtherActor :type Actor%20Object%20Reference)))

(event EventTick
  (params (DeltaSeconds :type Float%20%28single-precision%29)))

(fn ConstructionScript
  (bind _particlesystem (Variables|Default|GetParticleSystem))
  (bind _particlesystem_2 (Variables|Default|GetParticleSystem))
  (bind _particlesystem_3 (Variables|Default|GetParticleSystem))
  (bind _particlesystem_4 (Variables|Default|GetParticleSystem))
  (switch Utilities|FlowControl|Switch|SwitchondisplayCaseLongEnum (Variables|Default|GetDisplayCaseLongEnum)
    (:NewEnumerator0
      (Effects|Components|ParticleSystem|SetColorParameter _particlesystem_4 "ParticleColor1" (stale _output_get))
      (Effects|Components|ParticleSystem|SetColorParameter _particlesystem_4 "ParticleColor2" (stale _output_get)))
    (:NewEnumerator1
      (Effects|Components|ParticleSystem|SetColorParameter _particlesystem_3 "ParticleColor1" (stale _output_get))
      (Effects|Components|ParticleSystem|SetColorParameter _particlesystem_3 "ParticleColor2" (stale _output_get)))
    (:NewEnumerator2
      (Effects|Components|ParticleSystem|SetColorParameter _particlesystem_2 "ParticleColor1" (stale _output_get))
      (Effects|Components|ParticleSystem|SetColorParameter _particlesystem_2 "ParticleColor2" (stale _output_get)))
    (:NewEnumerator3
      (Effects|Components|ParticleSystem|SetColorParameter _particlesystem "ParticleColor1" (stale _output_get))
      (Effects|Components|ParticleSystem|SetColorParameter _particlesystem "ParticleColor2" (stale _output_get)))))