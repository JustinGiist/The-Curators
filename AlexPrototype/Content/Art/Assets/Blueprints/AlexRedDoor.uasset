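; Red keycard-style door that slides open with E while the player stands in its trigger box.
; On overlap it enables input and asks the overlapping actor's inventory for a "Red" item.
; The first successful press consumes that item and turns both lights green, after which E toggles the door freely.
; A timeline drives the door's relative location and plays its audio, reversing to undo the slide.
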(event OnComponentBeginOverlap(BoxCollision)
  (params (OtherActor :type Actor%20Object%20Reference) (OtherComp :type Primitive%20Component%20Object%20Reference) (OtherBodyIndex :type Integer) (bFromSweep :type Boolean) (SweepResult :type Hit%20Result%20Structure%20%28by%20ref%29))
  (Input|EnableInput (Game|GetPlayerController 0))
  (bind _pickedup (Class|InventorInterface|CheckInventory(Message) OtherActor "Red"))
  (if _pickedup
    (Variables|Default|SetCanOpen true)
    (else
      (Variables|Default|SetCanOpen false))))

(event OnComponentEndOverlap(BoxCollision)
  (params (OtherActor :type Actor%20Object%20Reference) (OtherComp :type Primitive%20Component%20Object%20Reference) (OtherBodyIndex :type Integer))
  (Input|DisableInput (Game|GetPlayerController 0)))

(event Input|KeyboardEvents|E
  (:Pressed
    (if (and (Variables|Default|GetCanOpen) (Variables|Default|GetCurrentlyRed))
      (Variables|Default|SetCurrentlyRed false)
      (Class|InventorInterface|RemovefromInventory(Message) (stale OnComponentBeginOverlap(BoxCollision) OtherActor) (Utilities|String|MakeLiteralString "Red"))
      (Variables|Default|SetDoorStatus true)
      (Rendering|Components|Light|SetLightColor (Variables|Default|GetFront) "(R=0.007843,G=1.000000,B=0.000000,A=1.000000)")
      (Rendering|Components|Light|SetLightColor (Variables|Default|GetBack) "(R=0.007843,G=1.000000,B=0.000000,A=1.000000)")
      ;[1 1 1] Door Opening/If door is set to green
      (if (Variables|Default|GetDoorStatus)
        (Variables|Default|SetDoorStatus false)
        (bind _door_swipe (Timeline|RedDoorTimeline Play)
          (:Update
            (Transformation|SetRelativeLocation (Variables|Default|GetDoor) _door_swipe false)
            (Audio|Components|Audio|Play (Variables|Default|GetAudio) 0.0)))
        (else
          (Variables|Default|SetDoorStatus true)
          (Timeline|RedDoorTimeline ReverseFromEnd)))
      (elif (Variables|Default|GetCanOpen)
        _))))

(event Input|KeyboardEvents|E
  ;[1 1 1] Door Opening/If door is set to green
  (:Pressed
    (if (not (Variables|Default|GetCurrentlyRed))
      (if (Variables|Default|GetDoorStatus)
        (Variables|Default|SetDoorStatus false)
        (bind _door_swipe (Timeline|RedDoorTimeline Play)
          (:Update
            (Transformation|SetRelativeLocation (Variables|Default|GetDoor) _door_swipe false)
            (Audio|Components|Audio|Play (Variables|Default|GetAudio) 0.0)))
        (else
          (Variables|Default|SetDoorStatus true)
          (Timeline|RedDoorTimeline ReverseFromEnd))))))

(fn ConstructionScript)