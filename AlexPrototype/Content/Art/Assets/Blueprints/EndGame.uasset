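; Exit door that ends the level once the overlapping actor holds the "Art" item.
; Overlapping DoorCollision queries that actor's inventory via an interface message, printing a prompt and enabling input on success, or a warning otherwise.
; While input is enabled, E opens the VerticalSlice level; leaving the volume disables input.
; The timeline door-swing logic is disconnected, and its own CheckInventory simply returns false.
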(event OnComponentBeginOverlap(DoorCollision)
  (params (OtherActor :type Actor%20Object%20Reference) (OtherComp :type Primitive%20Component%20Object%20Reference) (OtherBodyIndex :type Integer) (bFromSweep :type Boolean) (SweepResult :type Hit%20Result%20Structure%20%28by%20ref%29))
  (bind _returnvalue (Game|GetPlayerController 0))
  (bind _pickedup (Class|InventorInterface|CheckInventory(Message) OtherActor "Art"))
  (if _pickedup
    (Development|PrintString "Press E to Exit")
    (Input|EnableInput _returnvalue)
    (else
      (Development|PrintString "Obtain Art Piece Before Leaving")
      (Input|DisableInput _returnvalue))))

(event OnComponentEndOverlap(DoorCollision)
  (params (OtherActor :type Actor%20Object%20Reference) (OtherComp :type Primitive%20Component%20Object%20Reference) (OtherBodyIndex :type Integer))
  (Input|DisableInput (Game|GetPlayerController 0)))

(event Input|KeyboardEvents|E
  (:Pressed
    (Game|OpenLevel(byName) "VerticalSlice")))

(fn ConstructionScript)

(fn CheckInventory
  (params (Item :type String))
  (return false))