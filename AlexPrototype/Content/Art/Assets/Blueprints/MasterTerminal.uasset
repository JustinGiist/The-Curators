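; MasterTerminal is a hackable terminal that destroys a linked grid actor once the player has held the hack input long enough.
; Its collision box toggles input on overlap, and holding Hack or E sets the Erich character's hack flag and plays a looping-state sound until release.
; Tick compares summed gamepad and E key hold time to Hacktime, then destroys GridToDisable, disables interaction and swaps the screen material to look switched off.
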(event OnComponentBeginOverlap(CollisionBox)
  (params (OtherActor :type Actor%20Object%20Reference) (OtherComp :type Primitive%20Component%20Object%20Reference) (OtherBodyIndex :type Integer) (bFromSweep :type Boolean) (SweepResult :type Hit%20Result%20Structure%20%28by%20ref%29))
  (Input|EnableInput (Game|GetPlayerController 0)))

(event OnComponentEndOverlap(CollisionBox)
  (params (OtherActor :type Actor%20Object%20Reference) (OtherComp :type Primitive%20Component%20Object%20Reference) (OtherBodyIndex :type Integer))
  (Input|DisableInput (Game|GetPlayerController 0)))

(event EventTick
  (params (DeltaSeconds :type Float%20%28single-precision%29))
  (bind _returnvalue (Game|GetPlayerController 0))
  ;[1 1 1] Requires x amount of time before completeing
  (if (Variables|Default|GetCurrentlyHacking)
    (bind _output_get (Variables|Default|SetHoldtime (+ (Class|PlayerController|GetInputKeyTimeDown _returnvalue "Gamepad_FaceButton_Left") (Class|PlayerController|GetInputKeyTimeDown _returnvalue "E"))))
    (if (>= _output_get (Variables|Default|GetHacktime))
      (Variables|Default|SetInteractable false)
      (Variables|Default|SetCurrentlyHacking false)
      (Actor|DestroyActor (Variables|Default|GetGridToDisable))
      ;[1 1 1] "Turns the screen off"
      (Rendering|Material|SetMaterial (Variables|Default|GetTerminal) 0 "/Game/Blueprints/Assets/VerticalSliceAssets/characterAssets/character/ArmBraceRight_Material.ArmBraceRight_Material")
      (bind _aserich_final_char_combined (Utilities|Casting|CastToErichFinalCharCombined (Game|GetPlayerCharacter 0)))
      (Variables|/Game/Tech/ThirdPersonBP/Blueprints/ErichFinalCharCombined.ErichFinalCharCombined_C|SetHack _aserich_final_char_combined false)
      (Audio|Components|Audio|Stop (Variables|Default|GetHackingSound)))))

(event Input|ActionEvents|InputActionHack
  (bind _returnvalue (Game|GetPlayerCharacter 0))
  (bind _interactable (Variables|Default|GetInteractable))
  (bind _hackingsound (Variables|Default|GetHackingSound))
  (:Pressed
    (if _interactable
      (Variables|Default|SetCurrentlyHacking true)
      (bind _aserich_final_char_combined (Utilities|Casting|CastToErichFinalCharCombined _returnvalue))
      (Variables|/Game/Tech/ThirdPersonBP/Blueprints/ErichFinalCharCombined.ErichFinalCharCombined_C|SetHack _aserich_final_char_combined true)
      (Audio|Components|Audio|Play _hackingsound 0.0)))
  (:Released
    (if _interactable
      (Variables|Default|SetCurrentlyHacking false)
      (bind _aserich_final_char_combined_2 (Utilities|Casting|CastToErichFinalCharCombined _returnvalue))
      (Variables|/Game/Tech/ThirdPersonBP/Blueprints/ErichFinalCharCombined.ErichFinalCharCombined_C|SetHack _aserich_final_char_combined_2 false)
      (Audio|Components|Audio|Stop _hackingsound))))

(event Input|KeyboardEvents|E
  (bind _returnvalue (Game|GetPlayerCharacter 0))
  (bind _interactable (Variables|Default|GetInteractable))
  (bind _hackingsound (Variables|Default|GetHackingSound))
  (:Pressed
    (if _interactable
      (Variables|Default|SetCurrentlyHacking true)
      (bind _aserich_final_char_combined (Utilities|Casting|CastToErichFinalCharCombined _returnvalue))
      (Variables|/Game/Tech/ThirdPersonBP/Blueprints/ErichFinalCharCombined.ErichFinalCharCombined_C|SetHack _aserich_final_char_combined true)
      (Audio|Components|Audio|Play _hackingsound 0.0)))
  (:Released
    (if _interactable
      (Variables|Default|SetCurrentlyHacking false)
      (bind _aserich_final_char_combined_2 (Utilities|Casting|CastToErichFinalCharCombined _returnvalue))
      (Variables|/Game/Tech/ThirdPersonBP/Blueprints/ErichFinalCharCombined.ErichFinalCharCombined_C|SetHack _aserich_final_char_combined_2 false)
      (Audio|Components|Audio|Stop _hackingsound))))

(fn ConstructionScript)