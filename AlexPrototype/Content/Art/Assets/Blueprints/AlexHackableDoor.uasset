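; Yellow-locked sliding door that the player unlocks with a Yellow keycard or by holding E to hack it.
; A trigger box enables input and queries the overlapping actor's inventory for the card; a short E tap consumes it, while Tick checks hold time against HackTime for hacking.
; Either route turns both lights green and runs the door timeline, after which E toggles the door open and closed.
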(event OnComponentBeginOverlap(BoxCollision)
  (params (OtherActor :type Actor%20Object%20Reference) (OtherComp :type Primitive%20Component%20Object%20Reference) (OtherBodyIndex :type Integer) (bFromSweep :type Boolean) (SweepResult :type Hit%20Result%20Structure%20%28by%20ref%29))
  (Input|EnableInput (Game|GetPlayerController 0))
  (bind _pickedup (Class|InventorInterface|CheckInventory(Message) OtherActor "Yellow"))
  (if _pickedup
    (Variables|Default|SetCanUseKeycard true)
    (bind _inventory (Class|InventorInterface|GetInventory(Message) OtherActor))
    (Variables|Default|SetTemp%20Inventory _inventory)
    (else
      (Variables|Default|SetCanUseKeycard false))))

(event OnComponentEndOverlap(BoxCollision)
  (params (OtherActor :type Actor%20Object%20Reference) (OtherComp :type Primitive%20Component%20Object%20Reference) (OtherBodyIndex :type Integer))
  (Input|DisableInput (Game|GetPlayerController 0)))

(event EventTick
  (params (DeltaSeconds :type Float%20%28single-precision%29))
  ;[1 1 1] Regular Hack functionality. The Event tick needs to check hold time even when the player has a keycard. If the hold time check works in this comment box or the one above, it funnels back  to set currentlyYellow False and procceeds to door opening func
  (if (Variables|Default|GetCurrentlyHacking)
    (bind _output_get (Variables|Default|SetHoldTime (Class|PlayerController|GetInputKeyTimeDown (Game|GetPlayerController 0) "E")))
    (if (>= _output_get (Variables|Default|GetHackTime))
      (Variables|Default|SetCurrentlyHacking false)
      (Variables|Default|SetCurrentlyYellow false)
      (Variables|Default|SetDoorStatus true)
      (Rendering|Components|Light|SetLightColor (Variables|Default|GetFront) "(R=0.007843,G=1.000000,B=0.000000,A=1.000000)")
      (Rendering|Components|Light|SetLightColor (Variables|Default|GetBack) "(R=0.007843,G=1.000000,B=0.000000,A=1.000000)")
      ;[1 1 1] Door Opening/If door is set to green
      (if (Variables|Default|GetDoorStatus)
        (Variables|Default|SetDoorStatus false)
        (bind _doorswipe (Timeline|YellowDoorTimeline Play)
          (:Update
            (Transformation|SetRelativeLocation (Variables|Default|GetDoor) _doorswipe false)))
        (else
          (Variables|Default|SetDoorStatus true)
          (Timeline|YellowDoorTimeline ReverseFromEnd))))))

(event Input|KeyboardEvents|E
  (bind _temp_inventory (Variables|Default|GetTemp%20Inventory))
  ;[1 1 1] If player has keycard
  (:Pressed
    (if (and (Variables|Default|GetCanUseKeycard) (Variables|Default|GetCurrentlyYellow))
      (Variables|Default|SetCurrentlyHacking true)))
  (:Released
    (if (and (Variables|Default|GetCanUseKeycard) (Variables|Default|GetCurrentlyYellow))
      (Variables|Default|SetCurrentlyHacking false)
      (if (< (stale EventTick _output_get) 0.5)
        (Utilities|Array|RemoveIndex _temp_inventory (Utilities|Array|FindItem _temp_inventory (Utilities|String|MakeLiteralString "Yellow")))
        (Variables|Default|SetCanUseKeycard false)
        ;[1 1 1] Regular Hack functionality. The Event tick needs to check hold time even when the player has a keycard. If the hold time check works in this comment box or the one above, it funnels back  to set currentlyYellow False and procceeds to door opening func
        (Variables|Default|SetCurrentlyYellow false)
        (Variables|Default|SetDoorStatus true)
        (Rendering|Components|Light|SetLightColor (Variables|Default|GetFront) "(R=0.007843,G=1.000000,B=0.000000,A=1.000000)")
        (Rendering|Components|Light|SetLightColor (Variables|Default|GetBack) "(R=0.007843,G=1.000000,B=0.000000,A=1.000000)")
        ;[1 1 1] Door Opening/If door is set to green
        (if (Variables|Default|GetDoorStatus)
          (Variables|Default|SetDoorStatus false)
          (bind _doorswipe (Timeline|YellowDoorTimeline Play)
            (:Update
              (Transformation|SetRelativeLocation (Variables|Default|GetDoor) _doorswipe false)))
          (else
            (Variables|Default|SetDoorStatus true)
            (Timeline|YellowDoorTimeline ReverseFromEnd)))))))

(event Input|KeyboardEvents|E
  (bind _currentlyyellow (Variables|Default|GetCurrentlyYellow))
  ;[1 1 1] If Player doesn't have keycard
  (:Pressed
    (if _currentlyyellow
      (Variables|Default|SetCurrentlyHacking true)
      (Development|PrintString "CurrentlyHacking")))
  (:Released
    (if _currentlyyellow
      (Variables|Default|SetCurrentlyHacking false))))

(event Input|KeyboardEvents|E
  ;[1 1 1] Door Opening/If door is set to green
  (:Pressed
    (if (not (Variables|Default|GetCurrentlyYellow))
      (if (Variables|Default|GetDoorStatus)
        (Variables|Default|SetDoorStatus false)
        (bind _doorswipe (Timeline|YellowDoorTimeline Play)
          (:Update
            (Transformation|SetRelativeLocation (Variables|Default|GetDoor) _doorswipe false)))
        (else
          (Variables|Default|SetDoorStatus true)
          (Timeline|YellowDoorTimeline ReverseFromEnd))))))

(fn ConstructionScript)