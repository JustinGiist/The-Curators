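; Yellow keycard pickup that the player collects by walking into its box trigger.
; On overlap with the player pawn it sends an add-inventory message for "yellow", plays a pickup sound attached to the character's AltCamera and destroys itself.
; It then tells the PlayerHUD to add the yellow keycard.
; Its CheckInventory function is a stub that always returns false.
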(event OnComponentBeginOverlap(Box)
  (params (OtherActor :type Actor%20Object%20Reference) (OtherComp :type Primitive%20Component%20Object%20Reference) (OtherBodyIndex :type Integer) (bFromSweep :type Boolean) (SweepResult :type Hit%20Result%20Structure%20%28by%20ref%29))
  (if (== OtherActor (Game|Player|GetPlayerPawn 0))
    (Class|InventorInterface|AddInventory(Message) OtherActor "yellow")
    (bind _aserich_final_char_combined (Utilities|Casting|CastToErichFinalCharCombined OtherActor))
    (Class|GameplayStatics|PlaySoundAttached "/Game/Art/Assets/Sound/PickUp.PickUp" (Variables|/Game/Tech/ThirdPersonBP/Blueprints/ErichFinalCharCombined.ErichFinalCharCombined_C|GetAltCamera _aserich_final_char_combined))
    (Actor|DestroyActor)
    (bind _asplayer_hud (Utilities|Casting|CastToPlayerHUD (HUD|GetHUD (Game|GetPlayerController 0))))
    (Default|AddKeycardYellow _asplayer_hud)))

(fn ConstructionScript)

(fn CheckInventory
  (params (Item :type String))
  (return false))