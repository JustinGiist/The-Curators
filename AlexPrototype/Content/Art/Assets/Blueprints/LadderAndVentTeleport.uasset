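; An interactable ladder or vent that teleports the player character to a linked target when E is pressed.
; Overlapping the collision box toggles the actor's own input, so the key only responds nearby.
; Pressing E plays a vent or ladder sound chosen by a flag, disables character input and plays a fade Matinee.
; After a delay it teleports the character with zeroed rotation, then calls EnableInput on it.
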(event OnComponentBeginOverlap(CollisionBox)
  (params (OtherActor :type Actor%20Object%20Reference) (OtherComp :type Primitive%20Component%20Object%20Reference) (OtherBodyIndex :type Integer) (bFromSweep :type Boolean) (SweepResult :type Hit%20Result%20Structure%20%28by%20ref%29))
  (Input|EnableInput (Game|GetPlayerController 0)))

(event OnComponentEndOverlap(CollisionBox)
  (params (OtherActor :type Actor%20Object%20Reference) (OtherComp :type Primitive%20Component%20Object%20Reference) (OtherBodyIndex :type Integer))
  (Input|DisableInput (Game|GetPlayerController 0)))

(event Input|KeyboardEvents|E
  (bind _returnvalue (Game|GetPlayerCharacter 0))
  (:Pressed
    (if (Variables|Default|GetIsVent)
      (Audio|PlaySound2D "/Game/Assets/Sound/PlayerSounds/WalkTheVent.WalkTheVent")
      (else
        (Audio|PlaySound2D "/Game/Assets/Sound/PlayerSounds/Ladder.Ladder")))
    (Input|DisableInput _returnvalue (Game|GetPlayerController 0))
    (Audio|Components|Audio|Play (Variables|Default|GetFadeMatinee))
    (Utilities|FlowControl|Delay 1.0)
    (Transformation|Teleport _returnvalue (Transformation|GetActorLocation (Variables|Default|GetTeleportHere)) "0, 0, 0")
    (Utilities|FlowControl|Delay 0.25)
    (Input|EnableInput _returnvalue 0)))

(fn ConstructionScript)