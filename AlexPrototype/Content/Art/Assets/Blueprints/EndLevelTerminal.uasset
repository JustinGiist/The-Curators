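; EndLevelTerminal is a level-end trigger that reacts when the player pawn overlaps its Box component.
; The overlap plays the EndlevelMatinee sequence, then after a short delay disables player input and removes all widgets.
; A delayed load of the level named by NextLevelName is present but unconnected, so this Blueprint never changes level itself.
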(event OnComponentBeginOverlap(Box)
  (params (OtherActor :type Actor%20Object%20Reference) (OtherComp :type Primitive%20Component%20Object%20Reference) (OtherBodyIndex :type Integer) (bFromSweep :type Boolean) (SweepResult :type Hit%20Result%20Structure%20%28by%20ref%29))
  (if (== OtherActor (Game|Player|GetPlayerPawn 0))
    (Audio|Components|Audio|Play (Variables|Default|GetEndlevelMatinee))
    (Utilities|FlowControl|Delay 1.0)
    (Input|DisableInput (Game|GetPlayerCharacter 0) (Game|GetPlayerController 0))
    (Viewport|RemoveAllWidgets)))

(fn ConstructionScript)