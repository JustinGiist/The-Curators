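; Interactive locker actor whose hinged door the player opens and closes, exposing a pickup inside.
; A box collision enables input while the player pawn overlaps it, so Hack or E plays a sound and toggles the door.
; A timeline drives the door's yaw forward or in reverse, and its update sets CanPickUp after a short delay.
; Tick applies CanPickUp to the inner pickup's collision; closing never clears the flag.
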(event OnComponentBeginOverlap(BoxCollision)
  (params (OtherActor :type Actor%20Object%20Reference) (OtherComp :type Primitive%20Component%20Object%20Reference) (OtherBodyIndex :type Integer) (bFromSweep :type Boolean) (SweepResult :type Hit%20Result%20Structure%20%28by%20ref%29))
  (if (== OtherActor (Game|Player|GetPlayerPawn 0))
    (Input|EnableInput (Game|GetPlayerController 0))))

(event OnComponentEndOverlap(BoxCollision)
  (params (OtherActor :type Actor%20Object%20Reference) (OtherComp :type Primitive%20Component%20Object%20Reference) (OtherBodyIndex :type Integer))
  (if (== (Game|Player|GetPlayerPawn 0) OtherActor)
    (Input|DisableInput (Game|GetPlayerController 0))))

(event EventTick
  (params (DeltaSeconds :type Float%20%28single-precision%29))
  (Collision|SetActorEnableCollision (Variables|Default|GetPickUpInside) (Variables|Default|GetCanPickUp)))

(event Input|ActionEvents|InputActionHack
  (:Pressed
    (Audio|PlaySound2D "/Game/Assets/Sound/EnvironmentSounds/OpenLocker.OpenLocker")
    (if (Variables|Default|GetDoorStatus)
      (Variables|Default|SetDoorStatus false)
      (bind _locker_door_rot (Timeline|LockerDoorRotation Play)
        (:Update
          (Transformation|SetRelativeRotation (Variables|Default|GetLockerDoor) (Class|KismetMathLibrary|MakeRot 0.0 _locker_door_rot 0.0) false)
          (Utilities|FlowControl|Delay 0.5)
          (Variables|Default|SetCanPickUp true)))
      (else
        (Variables|Default|SetDoorStatus true)
        (Timeline|LockerDoorRotation Reverse)))))

(event Input|KeyboardEvents|E
  (:Pressed
    (Audio|PlaySound2D "/Game/Assets/Sound/EnvironmentSounds/OpenLocker.OpenLocker")
    (if (Variables|Default|GetDoorStatus)
      (Variables|Default|SetDoorStatus false)
      (bind _locker_door_rot (Timeline|LockerDoorRotation Play)
        (:Update
          (Transformation|SetRelativeRotation (Variables|Default|GetLockerDoor) (Class|KismetMathLibrary|MakeRot 0.0 _locker_door_rot 0.0) false)
          (Utilities|FlowControl|Delay 0.5)
          (Variables|Default|SetCanPickUp true)))
      (else
        (Variables|Default|SetDoorStatus true)
        (Timeline|LockerDoorRotation Reverse)))))

(fn ConstructionScript)