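; Short display case prop whose particle effect is tinted to match the game level it represents.
; The construction script switches on a case enum (Tutorial or Levels 1 to 3) and sets two color parameters on the particle component from that level's color pair.
; The event graph is empty, so the tint comes only from construction.
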(event EventBeginPlay)

(event Collision|EventActorBeginOverlap
  (params (OtherActor :type Actor%20Object%20Reference)))

(event EventTick
  (params (DeltaSeconds :type Float%20%28single-precision%29)))

(fn ConstructionScript
  (bind _p_displayparticleshort (Variables|Default|Getp_displayParticleShort))
  (bind _p_displayparticleshort_2 (Variables|Default|Getp_displayParticleShort))
  (bind _p_displayparticleshort_3 (Variables|Default|Getp_displayParticleShort))
  (bind _p_displayparticleshort_4 (Variables|Default|Getp_displayParticleShort))
  (switch Utilities|FlowControl|Switch|SwitchondisplayCaseShortEnum (Variables|Default|GetDisplayCaseShortEnum)
    (:NewEnumerator0
      (Effects|Components|ParticleSystem|SetColorParameter _p_displayparticleshort "ParticleColor1" (stale _output_get))
      (Effects|Components|ParticleSystem|SetColorParameter _p_displayparticleshort "ParticleColor2" (stale _output_get)))
    (:NewEnumerator1
      (Effects|Components|ParticleSystem|SetColorParameter _p_displayparticleshort_2 "ParticleColor1" (stale _output_get))
      (Effects|Components|ParticleSystem|SetColorParameter _p_displayparticleshort_2 "ParticleColor2" (stale _output_get)))
    (:NewEnumerator2
      (Effects|Components|ParticleSystem|SetColorParameter _p_displayparticleshort_3 "ParticleColor1" (stale _output_get))
      (Effects|Components|ParticleSystem|SetColorParameter _p_displayparticleshort_3 "ParticleColor2" (stale _output_get)))
    (:NewEnumerator3
      (Effects|Components|ParticleSystem|SetColorParameter _p_displayparticleshort_4 "ParticleColor1" (stale _output_get))
      (Effects|Components|ParticleSystem|SetColorParameter _p_displayparticleshort_4 "ParticleColor2" (stale _output_get)))))