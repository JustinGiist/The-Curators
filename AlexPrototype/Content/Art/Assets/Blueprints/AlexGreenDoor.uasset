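; Green sliding door actor that the player opens and closes with E while standing in its box trigger.
; Overlap begin and end on the box enable and disable input from player controller 0.
; Each press flips DoorStatus and either plays GreenDoorTimeLine or reverses it from the end.
; The timeline's DoorSwipe track drives the door's relative location, and every update restarts the audio.
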(event OnComponentBeginOverlap(BoxCollision)
  (params (OtherActor :type Actor%20Object%20Reference) (OtherComp :type Primitive%20Component%20Object%20Reference) (OtherBodyIndex :type Integer) (bFromSweep :type Boolean) (SweepResult :type Hit%20Result%20Structure%20%28by%20ref%29))
  (Input|EnableInput (Game|GetPlayerController 0)))

(event OnComponentEndOverlap(BoxCollision)
  (params (OtherActor :type Actor%20Object%20Reference) (OtherComp :type Primitive%20Component%20Object%20Reference) (OtherBodyIndex :type Integer))
  (Input|DisableInput (Game|GetPlayerController 0)))

(event Input|KeyboardEvents|E
  ;[1 1 1] Door Opening/If door is set to green
  (:Pressed
    (if (Variables|Default|GetDoorStatus)
      (Variables|Default|SetDoorStatus false)
      (bind _door_swipe (Timeline|GreenDoorTimeLine Play)
        (:Update
          (Transformation|SetRelativeLocation (Variables|Default|GetDoor) _door_swipe false)
          (Audio|Components|Audio|Play (Variables|Default|GetAudio) 0.0)))
      (else
        (Variables|Default|SetDoorStatus true)
        (Timeline|GreenDoorTimeLine ReverseFromEnd)))))

(fn ConstructionScript)