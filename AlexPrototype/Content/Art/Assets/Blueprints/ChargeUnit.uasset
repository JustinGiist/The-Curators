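; ChargeUnit is an interactable station that lets the player charge by holding E while overlapping its collision box.
; Overlap begin and end toggle input on the actor, with an on-screen debug prompt on entry.
; While E is held, Tick reads the key's hold time and calls UpdateCharge on the ThirdPersonCharacter.
; Releasing E clears the charging flag but re-enters the same hold-time check, allowing one further update.
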(event OnComponentBeginOverlap(CollisionBox)
  (params (OtherActor :type Actor%20Object%20Reference) (OtherComp :type Primitive%20Component%20Object%20Reference) (OtherBodyIndex :type Integer) (bFromSweep :type Boolean) (SweepResult :type Hit%20Result%20Structure%20%28by%20ref%29))
  (Input|EnableInput (Game|GetPlayerController 0))
  (Development|PrintString "Press E to Charge"))

(event OnComponentEndOverlap(CollisionBox)
  (params (OtherActor :type Actor%20Object%20Reference) (OtherComp :type Primitive%20Component%20Object%20Reference) (OtherBodyIndex :type Integer))
  (Input|DisableInput (Game|GetPlayerController 0)))

(event EventTick
  (params (DeltaSeconds :type Float%20%28single-precision%29))
  ;[1 1 1] Determines if Key is being Held Down
  (if (Variables|Default|GetIsCharging)
    (Variables|Default|SetHoldTime (Class|PlayerController|GetInputKeyTimeDown (Game|GetPlayerController 0) "E"))
    (if (> (Variables|Default|GetHoldTime) 0.0)
      ;[1 1 1] Call Update Charge Function Through CharacterController
      (bind _asthird_person_character (Utilities|Casting|CastToThirdPersonCharacter (Game|GetPlayerCharacter 0)))
      (Default|UpdateCharge _asthird_person_character))))

(event Input|KeyboardEvents|E
  ;[1 1 1] Call Update Charge Function Through CharacterController
  (:Pressed
    (Variables|Default|SetIsCharging true)
    (Development|PrintString "Charging"))
  (:Released
    (Variables|Default|SetIsCharging false)
    (if (> (Variables|Default|GetHoldTime) 0.0)
      (bind _asthird_person_character (Utilities|Casting|CastToThirdPersonCharacter (Game|GetPlayerCharacter 0)))
      (Default|UpdateCharge _asthird_person_character))))

(fn ConstructionScript)