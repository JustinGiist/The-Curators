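; Player HUD that draws a centered crosshair and, while Tab is held, an inventory panel with a title bar and item slots.
; Keycard functions set red, yellow and green flags; only red and yellow swap their slot for a card icon.
; DrawInventorySlot pairs each slot texture with a named hit box, whose clicks only print the name.
; CheckInventory is a stub that always returns false.
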(event EventDrawHUD
  (params (SizeX :type Integer) (SizeY :type Integer))
  (bind _returnvalue (Game|GetPlayerController 0))
  (bind _inventoryposx (Variables|Inventory|GetInventoryPosX))
  (bind _inventoryposy (Variables|Inventory|GetInventoryPosY))
  (bind _pixelseparation (Variables|Default|GetPixelSeparation))
  (bind _windowsbarh (Variables|Inventory|GetWindowsBarH))
  (bind _inventoryposy_2 (Variables|Inventory|GetInventoryPosY))
  (bind _inventoryposx_2 (Variables|Inventory|GetInventoryPosX))
  (bind _returnvalue_2 (+ _windowsbarh _inventoryposy_2 _pixelseparation))
  (Input|EnableInput (HUD|GetHUD _returnvalue) _returnvalue)
  ;[1 1 1] Draw Crosshairs
  (Class|HUD|DrawTextureSimple "/Game/Assets/FirstPersonBP/Textures/FirstPersonCrosshair.FirstPersonCrosshair" (Math|Conversions|ToFloat(Integer) (/ SizeX 2)) (Math|Conversions|ToFloat(Integer) (/ SizeY 2)) 1.0 false)
  ;[1 1 1] Create Player Inventory HUD
  (if (Variables|Default|GetIsHudCalled)
    (HUD|DrawRect "(R=0.120747,G=0.106758,B=0.735000,A=1.000000)" _inventoryposx _inventoryposy (Variables|Inventory|GetWindowsBarW) (Variables|Inventory|GetWindowsBarH))
    (HUD|DrawText "Inventory" "(R=0,G=0,B=0,A=1)" _inventoryposx _inventoryposy 0 1.0 false)
    (Class|HUD|AddHitBox (Math|Vector2D|MakeVector2D (Variables|Inventory|GetInventoryPosX) (Variables|Inventory|GetInventoryPosY)) (Math|Vector2D|MakeVector2D (Variables|Inventory|GetWindowsBarW) (Variables|Inventory|GetWindowsBarH)) "InventoryBar" false)
    (if (Variables|Default|GetKeyCard1)
      (Class|HUD|DrawTextureSimple "/Game/Assets/Textures/RedKeyCarde.RedKeyCarde" _inventoryposx_2 _returnvalue_2 1.0 false)
      (if (Variables|Default|GetKeyCardY)
        (Class|HUD|DrawTextureSimple "/Game/Assets/Textures/YellowKeyCard.YellowKeyCard" 5.6e+02 2.4e+02 1.0 false :!label _label)
        (else
          ;[1 1 1] Create Inventory Slots
          (Variables|Inventory|SetCurrentPosX _inventoryposx_2 :!label _label_2)
          (Variables|Inventory|SetCurrentPosY _returnvalue_2)
          (CallFunction|DrawInventorySlot (+ (Variables|Inventory|GetCurrentPosX) (Variables|Inventory|GetSlotSize) (Variables|Default|GetPixelSeparation)) (Variables|Inventory|GetCurrentPosY) "Slot2")))
      (else
        (CallFunction|DrawInventorySlot _inventoryposx_2 _returnvalue_2 "EmptyKey")
        (if (Variables|Default|GetKeyCardY)
          (goto _label)
          (else
            (goto _label_2)))))
    (Variables|Inventory|SetCurrentPosX (+ (Variables|Inventory|GetCurrentPosX) (Variables|Inventory|GetSlotSize) (Variables|Default|GetPixelSeparation)))
    (Variables|Inventory|SetCurrentPosY (Variables|Inventory|GetCurrentPosY))
    (CallFunction|DrawInventorySlot (+ (Variables|Inventory|GetCurrentPosX) (Variables|Inventory|GetSlotSize) (Variables|Default|GetPixelSeparation)) (Variables|Inventory|GetCurrentPosY) "Slot3")
    (CallFunction|DrawInventorySlot (Variables|Inventory|GetInventoryPosX) (+ (Variables|Default|GetPixelSeparation) (Variables|Inventory|GetWindowsBarH) (Variables|Default|GetSlotHeight)) "Slot4")
    (CallFunction|DrawInventorySlot (+ (Variables|Inventory|GetInventoryPosX) 3.7e+02) (+ (Variables|Default|GetPixelSeparation) (Variables|Inventory|GetWindowsBarH) (Variables|Default|GetSlotHeight)) "Slot5")))

(event EventHitBoxClick
  (params (BoxName :type Name))
  ;[1 1 1] Inventory Hit Box On Click Print
  (Development|PrintString (Utilities|String|ToString(Name) BoxName)))

(event Input|KeyboardEvents|Tab
  (bind _inventoryposx (Variables|Inventory|GetInventoryPosX))
  (bind _inventoryposy (Variables|Inventory|GetInventoryPosY))
  (bind _pixelseparation (Variables|Default|GetPixelSeparation))
  (bind _windowsbarh (Variables|Inventory|GetWindowsBarH))
  (bind _inventoryposy_2 (Variables|Inventory|GetInventoryPosY))
  (bind _inventoryposx_2 (Variables|Inventory|GetInventoryPosX))
  (bind _returnvalue (+ _windowsbarh _inventoryposy_2 _pixelseparation))
  (:Pressed
    ;[1 1 1] Create Player Inventory HUD
    (Variables|Default|SetIsHudCalled true)
    (if (Variables|Default|GetIsHudCalled) :!label _label
      (HUD|DrawRect "(R=0.120747,G=0.106758,B=0.735000,A=1.000000)" _inventoryposx _inventoryposy (Variables|Inventory|GetWindowsBarW) (Variables|Inventory|GetWindowsBarH))
      (HUD|DrawText "Inventory" "(R=0,G=0,B=0,A=1)" _inventoryposx _inventoryposy 0 1.0 false)
      (Class|HUD|AddHitBox (Math|Vector2D|MakeVector2D (Variables|Inventory|GetInventoryPosX) (Variables|Inventory|GetInventoryPosY)) (Math|Vector2D|MakeVector2D (Variables|Inventory|GetWindowsBarW) (Variables|Inventory|GetWindowsBarH)) "InventoryBar" false)
      (if (Variables|Default|GetKeyCard1)
        (Class|HUD|DrawTextureSimple "/Game/Assets/Textures/RedKeyCarde.RedKeyCarde" _inventoryposx_2 _returnvalue 1.0 false)
        (if (Variables|Default|GetKeyCardY)
          (Class|HUD|DrawTextureSimple "/Game/Assets/Textures/YellowKeyCard.YellowKeyCard" 5.6e+02 2.4e+02 1.0 false :!label _label_2)
          (else
            ;[1 1 1] Create Inventory Slots
            (Variables|Inventory|SetCurrentPosX _inventoryposx_2 :!label _label_3)
            (Variables|Inventory|SetCurrentPosY _returnvalue)
            (CallFunction|DrawInventorySlot (+ (Variables|Inventory|GetCurrentPosX) (Variables|Inventory|GetSlotSize) (Variables|Default|GetPixelSeparation)) (Variables|Inventory|GetCurrentPosY) "Slot2")))
        (else
          (CallFunction|DrawInventorySlot _inventoryposx_2 _returnvalue "EmptyKey")
          (if (Variables|Default|GetKeyCardY)
            (goto _label_2)
            (else
              (goto _label_3)))))
      (Variables|Inventory|SetCurrentPosX (+ (Variables|Inventory|GetCurrentPosX) (Variables|Inventory|GetSlotSize) (Variables|Default|GetPixelSeparation)))
      (Variables|Inventory|SetCurrentPosY (Variables|Inventory|GetCurrentPosY))
      (CallFunction|DrawInventorySlot (+ (Variables|Inventory|GetCurrentPosX) (Variables|Inventory|GetSlotSize) (Variables|Default|GetPixelSeparation)) (Variables|Inventory|GetCurrentPosY) "Slot3")
      (CallFunction|DrawInventorySlot (Variables|Inventory|GetInventoryPosX) (+ (Variables|Default|GetPixelSeparation) (Variables|Inventory|GetWindowsBarH) (Variables|Default|GetSlotHeight)) "Slot4")
      (CallFunction|DrawInventorySlot (+ (Variables|Inventory|GetInventoryPosX) 3.7e+02) (+ (Variables|Default|GetPixelSeparation) (Variables|Inventory|GetWindowsBarH) (Variables|Default|GetSlotHeight)) "Slot5")))
  (:Released
    (Variables|Default|SetIsHudCalled false)
    (goto _label)))

(fn ConstructionScript)

(fn DrawInventorySlot
  (params (PosX :type Float%20%28single-precision%29) (PosY :type Float%20%28single-precision%29) (SlotName :type Name))
  (bind _slotsize (Variables|Inventory|GetSlotSize))
  (Class|HUD|DrawTextureSimple "/Game/Assets/Textures/Black64x64.Black64x64" PosX PosY 1.0 false)
  (Class|HUD|AddHitBox (Math|Vector2D|MakeVector2D PosX PosY) (Math|Vector2D|MakeVector2D _slotsize _slotsize) SlotName false))

(fn AddKeycard
  (Variables|Default|SetKeyCard1 true))

(fn AddKeycardYellow
  (Variables|Default|SetKeyCardY true))

(fn AddKeycardGreen
  (Variables|Default|SetKeyCardG true))

(fn CheckInventory
  (params (Item :type String))
  (return false))