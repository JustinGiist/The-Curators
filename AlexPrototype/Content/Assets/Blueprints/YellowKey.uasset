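; YellowKey is a yellow keycard pickup that adds itself to the inventory of whatever overlaps its box.
; The overlap sends an AddInventory message tagged "yellow" to the other actor before any cast.
; Only for a ThirdPersonCharacter does it play the pickup sound on AltCamera, destroy itself and show the yellow keycard on PlayerHUD.
; CheckInventory is a stub returning false.
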(event OnComponentBeginOverlap(Box)
  (params (OtherActor :type Actor%20Object%20Reference) (OtherComp :type Primitive%20Component%20Object%20Reference) (OtherBodyIndex :type Integer) (bFromSweep :type Boolean) (SweepResult :type Hit%20Result%20Structure%20%28by%20ref%29))
  (Class|InventorInterface|AddInventory(Message) OtherActor "yellow")
  (bind _asthird_person_character (Utilities|Casting|CastToThirdPersonCharacter OtherActor))
  (Class|GameplayStatics|PlaySoundAttached "/Game/Assets/Sound/PickUp.PickUp" (Variables|/Game/ThirdPersonBP/Blueprints/ThirdPersonCharacter.ThirdPersonCharacter_C|GetAltCamera _asthird_person_character))
  (Actor|DestroyActor)
  (bind _asplayer_hud (Utilities|Casting|CastToPlayerHUD (HUD|GetHUD (Game|GetPlayerController 0))))
  (Default|AddKeycardYellow _asplayer_hud))

(event EventBeginPlay)

(event Collision|EventActorBeginOverlap
  (params (OtherActor :type Actor%20Object%20Reference)))

(event EventTick
  (params (DeltaSeconds :type Float%20%28single-precision%29)))

(fn ConstructionScript)

(fn CheckInventory
  (params (Item :type String))
  (return false))