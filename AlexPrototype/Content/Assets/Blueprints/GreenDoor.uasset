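; Door actor that the player can open and close with E, gated by a "green" keycard.
; On overlap it asks the overlapping actor's inventory for the card, then either toggles the press-E prompt and enables input, or toggles the keycard-needed prompt and disables input.
; E flips DoorStatus, plays an unlock sound at the character's AltCamera and runs a timeline forward or in reverse to drive door yaw.
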(event OnComponentEndOverlap(DoorCollision)
  (params (OtherActor :type Actor%20Object%20Reference) (OtherComp :type Primitive%20Component%20Object%20Reference) (OtherBodyIndex :type Integer))
  ;[1 1 1] Determine if player has keycard and allow input if so
  (Rendering|ToggleVisibility (Variables|Default|GetKeyCardNeeded) false)
  (Input|DisableInput (Game|GetPlayerController 0)))

(event OnComponentBeginOverlap(DoorCollision)
  (params (OtherActor :type Actor%20Object%20Reference) (OtherComp :type Primitive%20Component%20Object%20Reference) (OtherBodyIndex :type Integer) (bFromSweep :type Boolean) (SweepResult :type Hit%20Result%20Structure%20%28by%20ref%29))
  (bind _returnvalue (Game|GetPlayerController 0))
  ;[1 1 1] Determine if player has keycard and allow input if so
  (bind _pickedup (Class|InventorInterface|CheckInventory(Message) OtherActor "green"))
  (if _pickedup
    (Components|DestroyComponent (Variables|Default|GetKeyCardNeeded))
    (Rendering|ToggleVisibility (Variables|Default|GetPressE) false)
    (Input|EnableInput _returnvalue)
    (else
      (Rendering|ToggleVisibility (Variables|Default|GetKeyCardNeeded) false)
      (Input|DisableInput _returnvalue))))

(event Input|KeyboardEvents|E
  (:Pressed
    ;[1 1 1] On input rotate door
    (if (Variables|Default|Getdoor%20status)
      (Variables|Default|Setdoor%20status false)
      (Components|DestroyComponent (Variables|Default|GetPressE))
      (bind _asthird_person_character (Utilities|Casting|CastToThirdPersonCharacter (stale OnComponentBeginOverlap(DoorCollision) OtherActor)))
      (Class|GameplayStatics|PlaySoundAttached "/Game/Assets/Sound/Door_Unlock.Door_Unlock" (Variables|/Game/ThirdPersonBP/Blueprints/ThirdPersonCharacter.ThirdPersonCharacter_C|GetAltCamera _asthird_person_character))
      (bind _door_rot (Timeline|Timeline_0 Play)
        (:Update
          (Transformation|SetActorRelativeRotation (Class|KismetMathLibrary|MakeRot 0.0 _door_rot 0.0))))
      (else
        (Variables|Default|Setdoor%20status true)
        ;[1 1 1] Move to just after key press and delete other cast, more efficient
        (bind _asthird_person_character_2 (Utilities|Casting|CastToThirdPersonCharacter (stale OnComponentBeginOverlap(DoorCollision) OtherActor)))
        (Class|GameplayStatics|PlaySoundAttached "/Game/Assets/Sound/Door_Unlock.Door_Unlock" (Variables|/Game/ThirdPersonBP/Blueprints/ThirdPersonCharacter.ThirdPersonCharacter_C|GetAltCamera _asthird_person_character_2))
        (Timeline|Timeline_0 Reverse)))))

(fn ConstructionScript)

(fn CheckInventory
  (params (Item :type String))
  (return false))